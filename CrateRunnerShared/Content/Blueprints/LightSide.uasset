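; LightSide is a proximity light that changes brightness and colour when the PikeArmsFPCharacter player character is near it.
; Entering its Sphere plays a timeline that lerps the PointLight intensity between the Low and High variables and blends its colour between pink and pale yellow.
; Leaving the Sphere reverses the same timeline, so the light transitions back smoothly.
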(event OnComponentBeginOverlap(Sphere)
  (params (OtherActor :type Actor%20Object%20Reference) (OtherComp :type Primitive%20Component%20Object%20Reference) (OtherBodyIndex :type Integer) (bFromSweep :type Boolean) (SweepResult :type Hit%20Result%20Structure%20%28by%20ref%29))
  (Utilities|Casting|CastToPikeArmsFPCharacter OtherActor)
  (bind _brightness (Timeline|Timeline_0 Play)
    (:Update
      (Rendering|Components|Light|SetIntensity (Variables|Default|GetPointLight) (* (Math|Float|Lerp (Variables|Default|Getlow) (Variables|Default|Gethigh) _brightness) 1e+02))
      (Rendering|Components|Light|SetLightColor (Variables|Default|GetPointLight) (Math|Color|Lerp(LinearColor) "(R=0.970000,G=0.485000,B=0.534085,A=1.000000)" "(R=0.890000,G=0.858938,B=0.499920,A=1.000000)" (Math|Float|Lerp (Variables|Default|Getlow) (Variables|Default|Gethigh) _brightness)) true))))

(event OnComponentEndOverlap(Sphere)
  (params (OtherActor :type Actor%20Object%20Reference) (OtherComp :type Primitive%20Component%20Object%20Reference) (OtherBodyIndex :type Integer))
  (Utilities|Casting|CastToPikeArmsFPCharacter OtherActor)
  (bind _brightness (Timeline|Timeline_0 Reverse)
    (:Update
      (Rendering|Components|Light|SetIntensity (Variables|Default|GetPointLight) (* (Math|Float|Lerp (Variables|Default|Getlow) (Variables|Default|Gethigh) _brightness) 1e+02))
      (Rendering|Components|Light|SetLightColor (Variables|Default|GetPointLight) (Math|Color|Lerp(LinearColor) "(R=0.970000,G=0.485000,B=0.534085,A=1.000000)" "(R=0.890000,G=0.858938,B=0.499920,A=1.000000)" (Math|Float|Lerp (Variables|Default|Getlow) (Variables|Default|Gethigh) _brightness)) true))))

(event EventBeginPlay)

(event Collision|EventActorBeginOverlap
  (params (OtherActor :type Actor%20Object%20Reference)))

(event EventTick
  (params (DeltaSeconds :type Float%20%28single-precision%29)))

(fn ConstructionScript)