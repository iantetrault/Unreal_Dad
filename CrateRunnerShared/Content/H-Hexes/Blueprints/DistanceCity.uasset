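; DistanceCity is a city actor with two trigger-driven moving platforms: the HexvillageWell02 platform and a center lifter.
; When UnlockLift is set, overlapping their triggers turns a switch green, plays a sound, then after a delay runs a one-shot timeline lerp, lowering the well or raising the lifter.
; A third trigger reverses the lifter's timeline from its end without checking the unlock.
; The construction script places all three triggers at variable-defined world locations.
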(event OnComponentBeginOverlap(4oclockBox)
  (params (OtherActor :type Actor%20Object%20Reference) (OtherComp :type Primitive%20Component%20Object%20Reference) (OtherBodyIndex :type Integer) (bFromSweep :type Boolean) (SweepResult :type Hit%20Result%20Structure%20%28by%20ref%29))
  (bind _switcher_001 (Variables|Default|GetSwitcher_001))
  (if (Variables|Default|GetUnlockLift)
    (Rendering|Material|SetMaterial _switcher_001 0 "/Game/H-Hexes/Materials/SlidDoorMat/SteelDoor_Green.SteelDoor_Green")
    (Utilities|FlowControl|DoOnce false
      (:Completed
        (Audio|PlaySoundatLocation 0 "0, 0, 0")
        (Utilities|FlowControl|Delay 0.5)
        (Utilities|FlowControl|DoOnce false
          (:Completed
            (bind _dooropen (Timeline|Timeline_0 Play)
              (:Update
                (Transformation|SetRelativeLocation (Variables|Default|GetHex-village-_well02) (Math|Vector|Lerp(Vector) (Variables|Default|GetPlatformUp) (Variables|Default|GetPlatformDown) _dooropen) false false)))))))
    (else
      (Rendering|Material|SetMaterial _switcher_001 0 "/Game/H-Hexes/Materials/SlidDoorMat/SteelDoor_neutral.SteelDoor_neutral"))))

(event OnComponentBeginOverlap(Capsule)
  (params (OtherActor :type Actor%20Object%20Reference) (OtherComp :type Primitive%20Component%20Object%20Reference) (OtherBodyIndex :type Integer) (bFromSweep :type Boolean) (SweepResult :type Hit%20Result%20Structure%20%28by%20ref%29))
  (bind _switcher_001 (Variables|Default|GetSwitcher_001))
  (if (Variables|Default|GetUnlockLift)
    (Rendering|Material|SetMaterial _switcher_001 0 "/Game/H-Hexes/Materials/SlidDoorMat/SteelDoor_Green.SteelDoor_Green")
    (Utilities|FlowControl|DoOnce false
      (:Completed
        (Audio|PlaySoundatLocation 0 "0, 0, 0")
        (Utilities|FlowControl|Delay 2.0)
        (Utilities|FlowControl|DoOnce false
          (:Completed
            (bind _dooropen (Timeline|Timeline_1 Play)
              (:Update
                (Transformation|SetRelativeLocation (Variables|Default|GetCenterLifter) (Math|Vector|Lerp(Vector) (Variables|Default|GetcenterDown) (Variables|Default|GetcenterUp) _dooropen) false false)))))))
    (else
      (Rendering|Material|SetMaterial _switcher_001 0 "/Game/H-Hexes/Materials/SlidDoorMat/SteelDoor_neutral.SteelDoor_neutral"))))

(event OnComponentBeginOverlap(Capsule1)
  (params (OtherActor :type Actor%20Object%20Reference) (OtherComp :type Primitive%20Component%20Object%20Reference) (OtherBodyIndex :type Integer) (bFromSweep :type Boolean) (SweepResult :type Hit%20Result%20Structure%20%28by%20ref%29))
  (bind _dooropen (Timeline|Timeline_1 ReverseFromEnd)
    (:Update
      (Transformation|SetRelativeLocation (Variables|Default|GetCenterLifter) (Math|Vector|Lerp(Vector) (Variables|Default|GetcenterDown) (Variables|Default|GetcenterUp) _dooropen) false false))))

(event EventBeginPlay)

(event EventActorBeginOverlap
  (params (OtherActor :type Actor%20Object%20Reference)))

(event EventTick
  (params (DeltaSeconds :type Float%20%28single-precision%29)))

(fn ConstructionScript
  (Transformation|SetWorldLocation (Variables|Default|GetCapsule) (Variables|Default|GetUpSwitch) false false)
  (Transformation|SetWorldLocation (Variables|Default|GetCapsule1) (Variables|Default|GetDownSwitch) false false)
  (Transformation|SetWorldLocation (Variables|Default|Get4oclockBox) (Variables|Default|Get40clockPosition) false false))