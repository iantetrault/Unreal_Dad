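; Hex tile variant 8 Blueprint that configures its well and NGon mesh pieces in the Construction Script, with no active runtime logic.
; PerpCorridor, ParrellelCorridor and 6Blocker variables drive the Z scale of separate piece groups, and the Hexceiling mesh is set from HHex_Matrix.
; Var008Well02 and Var008NGon027 sit in both corridor groups, so the later ParrellelCorridor scale overrides PerpCorridor on them.
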(event EventBeginPlay)

(event EventActorBeginOverlap
  (params (OtherActor :type Actor%20Object%20Reference)))

(event EventTick
  (params (DeltaSeconds :type Float%20%28single-precision%29)))

(fn ConstructionScript
  (Transformation|SetRelativeScale3D (Variables|Default|GetVar-008_well05) (Math|Vector|MakeVector 1.0 1.0 (Variables|Default|GetPerpCorridor)))
  (Components|StaticMesh|SetStaticMesh (Variables|Default|GetHex-ceiling) "/Game/H-Hexes/M-Matrix/H-Hex_Matrix.H-Hex_Matrix")
  (Transformation|SetRelativeScale3D (Variables|Default|GetVar-008_well11) (Math|Vector|MakeVector 1.0 1.0 (Variables|Default|GetParrellelCorridor)))
  (Transformation|SetRelativeScale3D (Variables|Default|GetVar-008_well12) (Math|Vector|MakeVector 1.0 1.0 (Variables|Default|Get6Blocker))))